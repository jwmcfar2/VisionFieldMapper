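; Result render actor for the visual field test, drawing 2D result maps through widget components and a manually triggered scene capture.
; SetRefs and InvContrast store the result, contrast, color and shape data passed in.
; MakeResMap feeds that data to either the Result_Gen or ShapeColor_Analysis widget by ID, while SwapWidgets also hides the others and shows the chosen one.
; ForceCaptureScene captures ResultMapView on demand.
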(fn `ForceCaptureScene`
  (`SceneCaptureComponent2D.CaptureScene` (`self.ResultMap_View`)))

(fn `InvContrast`
  (params (ResMap :type "Array of /Game/VisualFieldTest/Results/TestResultsMapping Structure") (InvContrast :type Boolean))
  (set `self.ResMapRef` ResMap)
  (set `self.InvContrastRef` InvContrast))

(fn `MakeResMap`
  (switch `int` (`self.ResMapID`)
    (:`0`
      (`/Game/VisualFieldTest/Results/2D/Result_Gen.MakeResMap` (cast `/Game/VisualFieldTest/Results/2D/Result_Gen` (`WidgetComponent.GetWidget` (`self.ResultGen_Widget`)) :!pure true) (`self.ResMapRef`) (`self.InvContrastRef`)))
    (:`1`
      (`/Game/VisualFieldTest/Results/2D/ShapeColor_Analysis.MakeResMap` (cast `/Game/VisualFieldTest/Results/2D/ShapeColor_Analysis` (`WidgetComponent.GetWidget` (`self.ShapeColorAnalysis_Widget`)) :!pure true) (`self.ColorList`) (`self.ColorMapStruct`) (`self.ShapeList`) (`self.ShapeMapStruct`)))))

(fn `SetRefs`
  (params (ResMap :type "Array of /Game/VisualFieldTest/Results/TestResultsMapping Structure") (InvContrast :type Boolean) (ColorList :type "Array of LinearColor Structure") (ColorMapStruct :type "Array of /Game/VisualFieldTest/Results/ColorShapeMapStruct Structure") (ShapeList :type "Array of Texture2D Object Reference") (ShapeMapStruct :type "Array of /Game/VisualFieldTest/Results/ColorShapeMapStruct Structure"))
  (set `self.ResMapRef` ResMap)
  (set `self.InvContrastRef` InvContrast)
  (set `self.ColorList` ColorList)
  (set `self.ColorMapStruct` ColorMapStruct)
  (set `self.ShapeList` ShapeList)
  (set `self.ShapeMapStruct` ShapeMapStruct))

(fn `SwapWidgets`
  (params (newWidgetID :type Integer))
  (bind _shapecoloranalysis_widget (`self.ShapeColorAnalysis_Widget`))
  (bind _resultgen_widget (`self.ResultGen_Widget`))
  (`SceneComponent.SetVisibility` (`self.WidgetsRoot`) false true)
  (switch `int` newWidgetID
    (:`0`
      (`/Game/VisualFieldTest/Results/2D/Result_Gen.MakeResMap` (cast `/Game/VisualFieldTest/Results/2D/Result_Gen` (`WidgetComponent.GetWidget` _resultgen_widget) :!pure true) (`self.ResMapRef`) (`self.InvContrastRef`))
      (`SceneComponent.SetVisibility` _resultgen_widget true false))
    (:`1`
      (`/Game/VisualFieldTest/Results/2D/ShapeColor_Analysis.MakeResMap` (cast `/Game/VisualFieldTest/Results/2D/ShapeColor_Analysis` (`WidgetComponent.GetWidget` _shapecoloranalysis_widget) :!pure true) (`self.ColorList`) (`self.ColorMapStruct`) (`self.ShapeList`) (`self.ShapeMapStruct`))
      (`SceneComponent.SetVisibility` _shapecoloranalysis_widget true false))))

(fn `UserConstructionScript`)